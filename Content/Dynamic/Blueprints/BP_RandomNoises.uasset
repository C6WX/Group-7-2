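; BP_RandomNoises is a Blueprint meant to play random scary ambient sounds at irregular intervals, but as wired it plays nothing.
; BeginPlay calls PlayNoises, whose event body is empty, leaving the playback logic unreachable.
; That disconnected logic waits, picks between poltergeist and foley sounds, then loops through PlayNoises; a separate third branch has no sound assigned.
; Locations are raw random unit vectors, putting sounds near world origin.
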(event Custom|PlayNoises)

(event EventBeginPlay
  (CallFunction|PlayNoises))

(fn ConstructionScript)