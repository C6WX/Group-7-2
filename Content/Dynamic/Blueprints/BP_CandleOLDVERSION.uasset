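; BP_CandleOLDVERSION is an older candle actor that gives the player temporary light, toggling the character between candle and darkness states.
; Overlapping the Box lights the PointLight through a DoOnce, which resets after a random delay turns the candle off.
; Sphere overlaps call EnterCandle while lit and EnterDarkness on exit.
; Burnout does not notify the character, and the step disabling Sphere collision is disconnected.
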(event OnComponentBeginOverlap(Sphere)
  (params (OverlappedComponent :type Primitive%20Component%20Object%20Reference) (OtherActor :type Actor%20Object%20Reference) (OtherComp :type Primitive%20Component%20Object%20Reference) (OtherBodyIndex :type Integer) (bFromSweep :type Boolean) (SweepResult :type Hit%20Result%20Structure%20%28by%20ref%29))
  (Variables|Default|SetInSphereCollider true)
  (CallFunction|InActiveCandle))

(event OnComponentEndOverlap(Sphere)
  (params (OverlappedComponent :type Primitive%20Component%20Object%20Reference) (OtherActor :type Actor%20Object%20Reference) (OtherComp :type Primitive%20Component%20Object%20Reference) (OtherBodyIndex :type Integer))
  (Variables|Default|SetInSphereCollider false)
  (Variables|/Game/Dynamic/ThirdPerson/Blueprints/BP_ThirdPersonCharacter.BP_ThirdPersonCharacter_C|SetIn%20Darkness (stale Custom|InActiveCandle _asbp_third_person_character) true)
  (Default|EnterDarkness (stale Custom|InActiveCandle _asbp_third_person_character)))

(event OnComponentBeginOverlap(Box)
  (params (OverlappedComponent :type Primitive%20Component%20Object%20Reference) (OtherActor :type Actor%20Object%20Reference) (OtherComp :type Primitive%20Component%20Object%20Reference) (OtherBodyIndex :type Integer) (bFromSweep :type Boolean) (SweepResult :type Hit%20Result%20Structure%20%28by%20ref%29))
  (bind _asbp_third_person_character (Utilities|Casting|CastToBP_ThirdPersonCharacter OtherActor))
  (Utilities|FlowControl|DoOnce false
    (:Completed
      (Default|EnterCandle _asbp_third_person_character)
      (Variables|/Game/Dynamic/ThirdPerson/Blueprints/BP_ThirdPersonCharacter.BP_ThirdPersonCharacter_C|SetIn%20Darkness _asbp_third_person_character false)
      (Collision|SetCollisionEnabled (Variables|Default|GetSphere) "QueryOnly")
      (Rendering|SetVisibility (Variables|Default|GetPointLight) true false)
      (Variables|Default|SetCandleActive true)
      (Utilities|FlowControl|Delay (Math|Random|RandomFloatinRange 1e+01 3e+01)) ; after a random number of seconds within a range, the collision turns back off and the candle becomes invisable
      (Rendering|SetVisibility (Variables|Default|GetPointLight) false false)
      (Variables|Default|SetCandleActive false)
      (CallFunction|ResetCandleActivation))))

(event Custom|InActiveCandle
  (if (Variables|Default|GetInSphereCollider)
    (if (Variables|Default|GetCandleActive) ; as this only runs once, when the candle turns off, enter candle still runs
      (bind _asbp_third_person_character (Utilities|Casting|CastToBP_ThirdPersonCharacter (Game|GetPlayerCharacter 0)))
      (Variables|/Game/Dynamic/ThirdPerson/Blueprints/BP_ThirdPersonCharacter.BP_ThirdPersonCharacter_C|SetIn%20Darkness _asbp_third_person_character false)
      (Default|EnterCandle _asbp_third_person_character))))

(event Custom|ResetCandleActivation
  (Utilities|FlowControl|DoOnce false) ; enters at Reset
)

(event EventBeginPlay
  (Variables|Default|SetCandleActive false)
  (Rendering|SetVisibility (Variables|Default|GetPointLight) false false)
  (bind _returnvalue (Actor|GetActorOfClass "/Game/Dynamic/ThirdPerson/Blueprints/BP_ThirdPersonCharacter.BP_ThirdPersonCharacter_C"))
  (Variables|Default|SetCharacterReference _returnvalue))

(fn ConstructionScript)