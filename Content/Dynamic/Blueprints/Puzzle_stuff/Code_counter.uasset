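; Puzzle actor that shows which of the three code flags the player character holds, using pairs of cubes.
; All six cubes start hidden in game on BeginPlay.
; When BP_ThirdPersonCharacter begins overlapping, it reads Code1, Code2 and Code3 and unhides the matching pair for each true flag.
; Flags are checked only on overlap, and revealed cubes are never hidden again.
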(event EventBeginPlay
  (Development|SetHiddeninGame (Variables|Default|GetCube5) true false)
  (Development|SetHiddeninGame (Variables|Default|GetCube6) true false)
  (Development|SetHiddeninGame (Variables|Default|GetCube7) true false)
  (Development|SetHiddeninGame (Variables|Default|GetCube8) true false)
  (Development|SetHiddeninGame (Variables|Default|GetCube4) true false)
  (Development|SetHiddeninGame (Variables|Default|GetCube3) true false))

(event Collision|EventActorBeginOverlap
  (params (OtherActor :type Actor%20Object%20Reference))
  (bind _asbp_third_person_character (Utilities|Casting|CastToBP_ThirdPersonCharacter OtherActor))
  (if (Variables|/Game/Dynamic/ThirdPerson/Blueprints/BP_ThirdPersonCharacter.BP_ThirdPersonCharacter_C|GetCode%201 _asbp_third_person_character)
    (Development|SetHiddeninGame (Variables|Default|GetCube5) false false)
    (Development|SetHiddeninGame (Variables|Default|GetCube6) false false))
  (if (Variables|/Game/Dynamic/ThirdPerson/Blueprints/BP_ThirdPersonCharacter.BP_ThirdPersonCharacter_C|GetCode%202 _asbp_third_person_character)
    (Development|SetHiddeninGame (Variables|Default|GetCube7) false false)
    (Development|SetHiddeninGame (Variables|Default|GetCube8) false false))
  (if (Variables|/Game/Dynamic/ThirdPerson/Blueprints/BP_ThirdPersonCharacter.BP_ThirdPersonCharacter_C|GetCode%203 _asbp_third_person_character)
    (Development|SetHiddeninGame (Variables|Default|GetCube4) false false)
    (Development|SetHiddeninGame (Variables|Default|GetCube3) false false)))

(fn ConstructionScript)